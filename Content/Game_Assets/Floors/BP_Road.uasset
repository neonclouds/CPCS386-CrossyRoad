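; BP_Road is a road floor actor that spawns moving traffic from one of two ends, picked at random on BeginPlay.
; SpawnVehicle creates a random class from VehicleClasses when no valid Vehicle exists, sets its direction and speed, then starts a one-shot Delay timer.
; Two kill volumes, VehicleKill0 and VehicleKill1, destroy any BP_Vehicle that overlaps them.
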(event `self.ReceiveBeginPlay`
  (`parent.ReceiveBeginPlay`)
  (set `self.VehicleSpawnChoice` (`KismetMathLibrary.RandomInteger` 2))
  (`self.SpawnVehicle`))

(event `self.VehicleKill0.OnComponentBeginOverlap`
  (params (OverlappedComponent :type "PrimitiveComponent Object Reference") (OtherActor :type "Actor Object Reference") (OtherComp :type "PrimitiveComponent Object Reference") (OtherBodyIndex :type Integer) (bFromSweep :type Boolean) (SweepResult :type "HitResult Structure (by ref)"))
  (`KismetSystemLibrary.PrintString` "Destroying vehicle")
  (bind _asbp_vehicle (cast `/Game/Game_Assets/Vehicles/BP_Vehicle` OtherActor))
  (`self.K2_DestroyActor` _asbp_vehicle))

(event `self.VehicleKill1.OnComponentBeginOverlap`
  (params (OverlappedComponent :type "PrimitiveComponent Object Reference") (OtherActor :type "Actor Object Reference") (OtherComp :type "PrimitiveComponent Object Reference") (OtherBodyIndex :type Integer) (bFromSweep :type Boolean) (SweepResult :type "HitResult Structure (by ref)"))
  (`KismetSystemLibrary.PrintString` "Destroying vehicle")
  (bind _asbp_vehicle (cast `/Game/Game_Assets/Vehicles/BP_Vehicle` OtherActor))
  (`self.K2_DestroyActor` _asbp_vehicle))

(fn `OffsetLocation`
  (params (Original :type "Vector Structure") (OffsetX :type "Float (double-precision)") (OffsetY :type "Float (double-precision)") (OffsetZ :type "Float (double-precision)"))
  (returns (NewLocation :type "Vector Structure"))
  (return (`KismetMathLibrary.MakeVector` (+ (.x Original) OffsetX) (+ (.y Original) OffsetY) (+ (.z Original) OffsetZ))))

(fn `RandomVehicleClass`
  (returns (`Vehicle Class` :type "/Game/Game_Assets/Vehicles/BP_Vehicle Class Reference"))
  (bind _vehicleclasses (`self.VehicleClasses`))
  (return (`|GetArrayItem` _vehicleclasses (`KismetMathLibrary.RandomInteger` (`KismetArrayLibrary.Array_Length` _vehicleclasses)))))

(fn `SpawnVehicle`
  (`/Engine/EditorBlueprintResources/StandardMacros.IsValid` (`self.Vehicle`)
    (:`Is Not Valid`
      (if (> (`self.VehicleSpawnChoice`) 0)
        (bind _vehicle_class (`self.RandomVehicleClass`))
        (bind _returnvalue (`|SpawnActorFromClass` _vehicle_class (`KismetMathLibrary.MakeTransform` (`SceneComponent.K2_GetComponentLocation` (`self.VehicleSpawn1`)) (struct :`Yaw` -90.0)) "Undefined" "OverrideRootScale" null null))
        (set `/Game/Game_Assets/Vehicles/BP_Vehicle.Direction` -1.0 _returnvalue)
        (set `/Game/Game_Assets/Vehicles/BP_Vehicle.Speed` (`self.SpeedScale`) _returnvalue)
        (set `self.Vehicle` _returnvalue)
        (`KismetSystemLibrary.K2_SetTimerDelegate` (`|CreateDelegate` :!event `SpawnVehicle`) (`self.Delay`))
        (else
          (bind _vehicle_class_2 (`self.RandomVehicleClass`))
          (bind _returnvalue_2 (`|SpawnActorFromClass` _vehicle_class_2 (`KismetMathLibrary.MakeTransform` (`SceneComponent.K2_GetComponentLocation` (`self.VehicleSpawn0`)) (struct :`Yaw` 90.0)) "Undefined" "OverrideRootScale" null null))
          (set `/Game/Game_Assets/Vehicles/BP_Vehicle.Direction` -1.0 _returnvalue_2)
          (set `/Game/Game_Assets/Vehicles/BP_Vehicle.Speed` (`self.SpeedScale`) _returnvalue_2)
          (set `self.Vehicle` _returnvalue_2)
          (`KismetSystemLibrary.K2_SetTimerDelegate` (`|CreateDelegate` :!event `SpawnVehicle`) (`self.Delay`)))))))

(fn `UserConstructionScript`
  (`parent.UserConstructionScript`)
  (`KismetSystemLibrary.PrintString` "Constructing Road"))